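; Manages a destructible ship built from shattered mesh pieces that break away when stood on or hit by random explosions.
; Construction fills a map of health per piece, which standing events and a self-rescheduling random explosion timer reduce.
; Falling health drives destruction material parameters on each piece.
; At zero health, a piece loses collision and a timeline moves and rotates it before it is hidden and destroyed.
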(event Custom|Start%20Random%20Destroying
  (CallFunction|RandomExplosion))

(event Custom|LetPieceVanish
  (params (Piece :type Static%20Mesh%20Component%20Object%20Reference))
  (Collision|SetCollisionEnabled Piece "NoCollision")
  (bind (_direction _flying _rotation) (Timeline|Timeline_0 PlayFromStart)
    (:Update
      (Transformation|SetRelativeLocation Piece (- (Variables|/Script/Engine.SceneComponent|GetRelativeLocation Piece) (* (+ _flying (Math|Vector|MakeVector 0.0 (Math|Random|RandomFloatinRange 0.5 -0.5) 0.0)) 8.0)) true true)
      (Transformation|SetRelativeRotation Piece (Math|Conversions|RotationFromXVector _rotation) false false))
    (:Finished
      (Development|SetHiddeninGame Piece true false)
      (Components|DestroyComponent Piece))))

(event EventBeginPlay)

(event Collision|EventActorBeginOverlap
  (params (OtherActor :type Actor%20Object%20Reference)))

(event EventTick
  (params (DeltaSeconds :type Float%20%28single-precision%29)))

(event EventStandingonWhichPiece
  (params (Piece :type Static%20Mesh%20Component%20Object%20Reference))
  (bind _piecescollection (Variables|Default|GetPiecesCollection))
  (bind (_value _returnvalue) (Utilities|Map|Find _piecescollection Piece))
  (bind _returnvalue_2 (- _value 5))
  (if _returnvalue
    (if (== _returnvalue_2 0)
      (CallFunction|PieceDeath Piece)
      (else
        (Utilities|Map|Add _piecescollection Piece _returnvalue_2)
        (CallFunction|ShowDestrctuionLevel _returnvalue_2 Piece)))))

(fn ConstructionScript
  (CallFunction|PreparePieces))

(fn PreparePieces
  (bind _output_get (Variables|Default|SetAll%20Pieces (Utilities|Array|MakeArray (Variables|Default|GetSM_Shatter_Test2_polySurface245) (Variables|Default|GetSM_Shatter_Test2_polySurface154) (Variables|Default|GetSM_Shatter_Test2_polySurface164) (Variables|Default|GetSM_Shatter_Test2_polySurface167) (Variables|Default|GetSM_Shatter_Test2_polySurface171) (Variables|Default|GetSM_Shatter_Test2_polySurface175) (Variables|Default|GetSM_Shatter_Test2_polySurface176) (Variables|Default|GetSM_Shatter_Test2_polySurface177) (Variables|Default|GetSM_Shatter_Test2_polySurface178) (Variables|Default|GetSM_Shatter_Test2_polySurface179) (Variables|Default|GetSM_Shatter_Test2_polySurface185) (Variables|Default|GetSM_Shatter_Test2_polySurface187) (Variables|Default|GetSM_Shatter_Test2_polySurface188) (Variables|Default|GetSM_Shatter_Test2_polySurface191) (Variables|Default|GetSM_Shatter_Test2_polySurface192) (Variables|Default|GetSM_Shatter_Test2_polySurface194) (Variables|Default|GetSM_Shatter_Test2_polySurface197) (Variables|Default|GetSM_Shatter_Test2_polySurface200) (Variables|Default|GetSM_Shatter_Test2_polySurface204) (Variables|Default|GetSM_Shatter_Test2_polySurface205) (Variables|Default|GetSM_Shatter_Test2_polySurface207) (Variables|Default|GetSM_Shatter_Test2_polySurface210) (Variables|Default|GetSM_Shatter_Test2_polySurface219) (Variables|Default|GetSM_Shatter_Test2_polySurface220) (Variables|Default|GetSM_Shatter_Test2_polySurface226) (Variables|Default|GetSM_Shatter_Test2_polySurface229) (Variables|Default|GetSM_Shatter_Test2_polySurface232) (Variables|Default|GetSM_Shatter_Test2_polySurface235) (Variables|Default|GetSM_Shatter_Test2_side2_polySurface84) (Variables|Default|GetSM_Shatter_Test2_polySurface239) (Variables|Default|GetSM_Shatter_Test2_polySurface241) (Variables|Default|GetSM_Shatter_Test2_side2_polySurface86) (Variables|Default|GetSM_Shatter_Test2_polySurface246) (Variables|Default|GetSM_Shatter_Test2_polySurface249) (Variables|Default|GetSM_Shatter_Test2_polySurface253) (Variables|Default|GetSM_Shatter_Test2_polySurface255) (Variables|Default|GetSM_Shatter_Test2_polySurface259) (Variables|Default|GetSM_Shatter_Test2_polySurface268) (Variables|Default|GetSM_Shatter_Test2_polySurface269) (Variables|Default|GetSM_Shatter_Test2_polySurface270) (Variables|Default|GetSM_Shatter_Test2_polySurface271) (Variables|Default|GetSM_Shatter_Test2_polySurface272) (Variables|Default|GetSM_Shatter_Test2_polySurface273) (Variables|Default|GetSM_Shatter_Test2_polySurface274) (Variables|Default|GetSM_Shatter_Test2_polySurface275) (Variables|Default|GetSM_Shatter_Test2_polySurface276) (Variables|Default|GetSM_Shatter_Test2_polySurface277) (Variables|Default|GetSM_Shatter_Test2_polySurface278) (Variables|Default|GetSM_Shatter_Test2_polySurface279) (Variables|Default|GetSM_Shatter_Test2_polySurface280) (Variables|Default|GetSM_Shatter_Test2_polySurface281) (Variables|Default|GetSM_Shatter_Test2_polySurface282) (Variables|Default|GetSM_Shatter_Test2_polySurface283) (Variables|Default|GetSM_Shatter_Test2_polySurface284) (Variables|Default|GetSM_Shatter_Test2_polySurface78) (Variables|Default|GetSM_Shatter_Test2_polySurface90) (Variables|Default|GetSM_Shatter_Test2_side2_polySurface69) (Variables|Default|GetSM_Shatter_Test2_side2_polySurface72) (Variables|Default|GetSM_Shatter_Test2_side2_polySurface75) (Variables|Default|GetSM_Shatter_Test2_side2_polySurface78) (Variables|Default|GetSM_Shatter_Test2_side2_polySurface81))))
  (for _array_element _output_get
    (Utilities|Map|Add (Variables|Default|GetPiecesCollection) _array_element 100)))

(fn RandomExplosion
  (bind _piecescollection (Variables|Default|GetPiecesCollection))
  (bind _all_pieces (Variables|Default|GetAll%20Pieces))
  (bind _output_get (LocalVariables|SetCurrentPiece (Utilities|Array|Get(acopy) _all_pieces (Math|Random|RandomIntegerinRange 0 (- (Utilities|Array|Length _all_pieces) 1)))))
  (Utilities|IsValid _output_get
    (:Is%20Valid
      (LocalVariables|SetCurrentDamage (Math|Random|RandomIntegerinRange 40 40))
      (if (.ReturnValue (Utilities|Map|Find _piecescollection (LocalVariables|GetCurrentPiece)))
        (Utilities|Map|Add _piecescollection (LocalVariables|GetCurrentPiece) (- (.Value (Utilities|Map|Find _piecescollection (LocalVariables|GetCurrentPiece))) (LocalVariables|GetCurrentDamage)))
        (CallFunction|ShowDestrctuionLevel (.Value (Utilities|Map|Find _piecescollection (LocalVariables|GetCurrentPiece))) (LocalVariables|GetCurrentPiece))
        (Utilities|IsValid (LocalVariables|GetCurrentPiece)
          (:Is%20Valid
            (Effects|SpawnEmitteratLocation "/Game/StarterContent/Particles/P_Explosion.P_Explosion" (+ (Transformation|GetWorldLocation (LocalVariables|GetCurrentPiece)) "0, 0,60.000000"))))))
    (:Is%20Not%20Valid
      _))
  (Utilities|Time|SetTimerbyFunctionName 0 "Random Explosion" (Math|Random|RandomFloatinRange 0.1 1.0)))

(fn PieceDeath
  (params (Piece :type Static%20Mesh%20Component%20Object%20Reference))
  (CallFunction|LetPieceVanish Piece))

(fn ShowDestrctuionLevel
  (params (Health :type Integer) (Piece :type Static%20Mesh%20Component%20Object%20Reference))
  (Math|Integer|CompareInt Health 60
    (:<
      (Math|Integer|CompareInt Health 30
        (:>
          (Rendering|Material|SetScalarParameterValueonMaterials Piece "Destruction" 0.6)
          (Rendering|Material|SetScalarParameterValueonMaterials Piece "Edge" 0.05 :!label _label))
        (:<
          (if (<= Health 0)
            (CallFunction|PieceDeath Piece)
            (else
              (Rendering|Material|SetScalarParameterValueonMaterials Piece "Destruction" 0.2)
              (goto _label))))))))