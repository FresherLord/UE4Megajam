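; Game mode for SpaceCats local multiplayer with drop-in joining for up to four players before the game starts.
; BeginPlay creates four local players with IDs and shows the start screen.
; Join and remove events swap each controller between InitPawn and a ThirdPersonCharacter, update the screen and keep the view on MainCamera.
; Starting the game activates listed characters, flags their index-matched controllers as running, calls StartingGame and notifies the screen.
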(event Custom|Add%20Player
  (params (Player :type Third%20Person%20Character%20Object%20Reference))
  (Utilities|Array|Add (Variables|Default|GetPlayer) Player))

(event Custom|Remove%20Player
  (params (Controller :type Player%20Controller%20Object%20Reference))
  (bind _returnvalue (Pawn|GetControlledPawn Controller))
  (bind _spawn_points (Variables|Default|GetSpawn%20Points))
  (Utilities|IsValid _returnvalue
    (:Is%20Valid
      (Actor|DestroyActor _returnvalue)
      (bind _asplayer_controller_atro_cats (Utilities|Casting|CastToPlayerControllerAtroCats Controller))
      (Default|PlayerDissconected (Variables|Default|GetStartScreen) (Variables|/Game/BP/PlayerControllerAtroCats.PlayerControllerAtroCats_C|GetID _asplayer_controller_atro_cats))
      (bind _returnvalue_2 (Game|SpawnActorfromClass "/Game/BP/InitPawn.InitPawn_C" (Transformation|GetActorTransform (Utilities|Array|Get(acopy) _spawn_points (Math|Random|RandomIntegerinRange 0 (- (Utilities|Array|Length _spawn_points) 1)))) "Undefined" 0 0))
      (Pawn|Possess Controller _returnvalue_2)
      (Game|Player|SetViewTargetwithBlend Controller (Variables|Default|GetmainCamera) 0.0 "VTBlend_Linear" 0.0 false))))

(event Custom|Starting%20Game_Event
  (for (_array_element _array_index) (Variables|Default|GetPlayer)
    (Default|Activate _array_element)
    (Development|PrintString (Utilities|GetDisplayName (Utilities|Array|Get(acopy) (Variables|Default|GetPlayerController) _array_index)))
    (Variables|/Game/BP/PlayerControllerAtroCats.PlayerControllerAtroCats_C|SetisGameSessionRunning (Utilities|Array|Get(acopy) (Variables|Default|GetPlayerController) _array_index) true))
  (Default|CallStartingGame)
  (Default|StartGame (Variables|Default|GetStartScreen)))

(event Custom|Player%20Join
  (params (Controller :type Player%20Controller%20Object%20Reference))
  (bind _returnvalue (Pawn|GetControlledPawn Controller))
  (Utilities|IsValid _returnvalue
    (:Is%20Valid
      (Actor|DestroyActor _returnvalue)
      (bind _asplayer_controller_atro_cats (Utilities|Casting|CastToPlayerControllerAtroCats Controller))
      (Default|PlayerJoined (Variables|Default|GetStartScreen) (Variables|/Game/BP/PlayerControllerAtroCats.PlayerControllerAtroCats_C|GetID _asplayer_controller_atro_cats))
      (bind _returnvalue_2 (Game|SpawnActorfromClass "/Game/ThirdPersonBP/Blueprints/ThirdPersonCharacter.ThirdPersonCharacter_C" (Transformation|GetActorTransform (Utilities|Array|Get(acopy) (Variables|Default|GetSpawn%20Points) (Variables|/Game/BP/PlayerControllerAtroCats.PlayerControllerAtroCats_C|GetID _asplayer_controller_atro_cats))) "Undefined" 0 0))
      (CallFunction|AddPlayer _returnvalue_2)
      (Pawn|Possess Controller _returnvalue_2)
      (Game|Player|SetViewTargetwithBlend Controller (Variables|Default|GetmainCamera) 0.0 "VTBlend_Linear" 0.0 false))))

(event EventBeginPlay
  (bind _outactors (Actor|GetAllActorsOfClass "/Script/Engine.PlayerStart"))
  (Variables|Default|SetSpawn%20Points _outactors)
  (Utilities|FlowControl|Sequence
    (:then_0
      (bind _returnvalue (Class|GameplayStatics|CreatePlayer -1))
      (bind _asplayer_controller_atro_cats (Utilities|Casting|CastToPlayerControllerAtroCats _returnvalue))
      (Utilities|Array|Add (Variables|Default|GetPlayerController) _asplayer_controller_atro_cats)
      (Variables|/Game/BP/PlayerControllerAtroCats.PlayerControllerAtroCats_C|SetID _asplayer_controller_atro_cats 0)
      (bind _returnvalue_2 (UserInterface|CreateWidget "/Game/BP/UMG_StartSCreen.UMG_StartScreen_C"))
      (bind _output_get (Variables|Default|SetStartScreen _returnvalue_2))
      (UserInterface|Viewport|AddtoViewport _output_get 0))
    (:then_1
      (bind _returnvalue_3 (Class|GameplayStatics|CreatePlayer -1))
      (bind _asplayer_controller_atro_cats_2 (Utilities|Casting|CastToPlayerControllerAtroCats _returnvalue_3))
      (Variables|/Game/BP/PlayerControllerAtroCats.PlayerControllerAtroCats_C|SetID _asplayer_controller_atro_cats_2 1)
      (Utilities|Array|Add (Variables|Default|GetPlayerController) _asplayer_controller_atro_cats_2))
    (:then_2
      (bind _returnvalue_4 (Class|GameplayStatics|CreatePlayer -1))
      (bind _asplayer_controller_atro_cats_3 (Utilities|Casting|CastToPlayerControllerAtroCats _returnvalue_4))
      (Variables|/Game/BP/PlayerControllerAtroCats.PlayerControllerAtroCats_C|SetID _asplayer_controller_atro_cats_3 2)
      (Utilities|Array|Add (Variables|Default|GetPlayerController) _asplayer_controller_atro_cats_3))
    (:then_3
      ;[1 1 1] Fail??
      (bind _returnvalue_5 (Class|GameplayStatics|CreatePlayer -1))
      (bind _asplayer_controller_atro_cats_4 (Utilities|Casting|CastToPlayerControllerAtroCats _returnvalue_5))
      (Variables|/Game/BP/PlayerControllerAtroCats.PlayerControllerAtroCats_C|SetID _asplayer_controller_atro_cats_4 3)
      (Utilities|Array|Add (Variables|Default|GetPlayerController) _asplayer_controller_atro_cats_4))))

(event EventTick
  (params (DeltaSeconds :type Float%20%28single-precision%29)))

(fn ConstructionScript)