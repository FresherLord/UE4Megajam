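; Manages the destructible static mesh pieces of a ship, keeping a health value per piece in a map built by the construction script.
; StandingonWhichPiece drains the given piece, while StartRandomDestroying begins a self-rescheduling timer that explodes and damages random pieces.
; Lower health changes material Destruction and Edge parameters to show wear.
; At zero health a piece loses collision, moves and rotates on a timeline, then hides and is destroyed.
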(event Custom|Start%20Random%20Destroying
  (CallFunction|RandomExplosion))

(event Custom|LetPieceVanish
  (params (Piece :type Static%20Mesh%20Component%20Object%20Reference))
  (Collision|SetCollisionEnabled Piece "NoCollision")
  (bind (_direction _flying _rotation) (Timeline|Timeline_0 PlayFromStart)
    (:Update
      (Transformation|SetRelativeLocation Piece (- (Variables|/Script/Engine.SceneComponent|GetRelativeLocation Piece) (* (+ _flying (Math|Vector|MakeVector 0.0 (Math|Random|RandomFloatinRange 0.5 -0.5) 0.0)) 8.0)) true true)
      (Transformation|SetRelativeRotation Piece (Math|Conversions|RotationFromXVector _rotation) false false))
    (:Finished
      (Development|SetHiddeninGame Piece true false)
      (Components|DestroyComponent Piece))))

(event EventBeginPlay)

(event Collision|EventActorBeginOverlap
  (params (OtherActor :type Actor%20Object%20Reference)))

(event EventTick
  (params (DeltaSeconds :type Float%20%28single-precision%29)))

(event EventStandingonWhichPiece
  (params (Piece :type Static%20Mesh%20Component%20Object%20Reference))
  (bind _piecescollection (Variables|Default|GetPiecesCollection))
  (bind (_value _returnvalue) (Utilities|Map|Find _piecescollection Piece))
  (bind _returnvalue_2 (- _value 5))
  (if _returnvalue
    (if (== _returnvalue_2 0)
      (CallFunction|PieceDeath Piece)
      (else
        (Utilities|Map|Add _piecescollection Piece _returnvalue_2)
        (CallFunction|ShowDestrctuionLevel _returnvalue_2 Piece)))))

(fn ConstructionScript
  (CallFunction|PreparePieces))

(fn PreparePieces
  (bind _output_get (Variables|Default|SetAll%20Pieces (Utilities|Array|MakeArray (Variables|Default|GetStaticMesh1) (Variables|Default|GetStaticMesh2) (Variables|Default|GetStaticMesh3) (Variables|Default|GetStaticMesh))))
  (for _array_element _output_get
    (Utilities|Map|Add (Variables|Default|GetPiecesCollection) _array_element 100)))

(fn RandomExplosion
  (bind _piecescollection (Variables|Default|GetPiecesCollection))
  (bind _all_pieces (Variables|Default|GetAll%20Pieces))
  (bind _output_get (LocalVariables|SetCurrentPiece (Utilities|Array|Get(acopy) _all_pieces (Math|Random|RandomIntegerinRange 0 (- (Utilities|Array|Length _all_pieces) 1)))))
  (Utilities|IsValid _output_get
    (:Is%20Valid
      (LocalVariables|SetCurrentDamage (Math|Random|RandomIntegerinRange 30 50))
      (if (.ReturnValue (Utilities|Map|Find _piecescollection (LocalVariables|GetCurrentPiece)))
        (Utilities|Map|Add _piecescollection (LocalVariables|GetCurrentPiece) (- (.Value (Utilities|Map|Find _piecescollection (LocalVariables|GetCurrentPiece))) (LocalVariables|GetCurrentDamage)))
        (CallFunction|ShowDestrctuionLevel (.Value (Utilities|Map|Find _piecescollection (LocalVariables|GetCurrentPiece))) (LocalVariables|GetCurrentPiece))
        (Utilities|IsValid (LocalVariables|GetCurrentPiece)
          (:Is%20Valid
            (Effects|SpawnEmitteratLocation "/Game/StarterContent/Particles/P_Explosion.P_Explosion" (+ (Transformation|GetWorldLocation (LocalVariables|GetCurrentPiece)) "0, 0,60.000000"))))))
    (:Is%20Not%20Valid
      _))
  (Utilities|Time|SetTimerbyFunctionName 0 "Random Explosion" (Math|Random|RandomFloatinRange 5.0 1e+01)))

(fn PieceDeath
  (params (Piece :type Static%20Mesh%20Component%20Object%20Reference))
  (CallFunction|LetPieceVanish Piece))

(fn ShowDestrctuionLevel
  (params (Health :type Integer) (Piece :type Static%20Mesh%20Component%20Object%20Reference))
  (Math|Integer|CompareInt Health 50
    (:<
      (Math|Integer|CompareInt Health 25
        (:>
          (Rendering|Material|SetScalarParameterValueonMaterials Piece "Destruction" 0.7)
          (Rendering|Material|SetScalarParameterValueonMaterials Piece "Edge" 0.05 :!label _label))
        (:<
          (if (<= Health 0)
            (CallFunction|PieceDeath Piece)
            (else
              (Rendering|Material|SetScalarParameterValueonMaterials Piece "Destruction" 0.5)
              (goto _label))))))))